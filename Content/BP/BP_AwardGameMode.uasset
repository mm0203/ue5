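; BP_AwardGameMode is a game mode Blueprint that respawns the player when the player pawn is destroyed.
; On BeginPlay it binds a handler to player 0's pawn OnDestroyed event.
; The handler spawns a new BP_Award at the player start's transform, has the player controller possess it, then rebinds to the new pawn so respawning repeats.
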(event `self.ReceiveBeginPlay`
  (`self.RespawnEvent`))

(event `RespawnEvent`
  ;[1 1 1] 復活処理
  (add `self.OnDestroyed` (`GameplayStatics.GetPlayerPawn` 0) (delegate `RespawnAward`)) ; プレイヤーが死んだら
)

(event `RespawnAward` :!signature `self.OnDestroyed`
  (params (DestroyedActor :type "Actor Object Reference"))
  ;[1 1 1] 復活処理
  (bind _returnvalue (`|SpawnActorFromClass` "/Game/BP/BP_Award.BP_Award_C" (`self.GetTransform` (`self.K2_FindPlayerStart` null)) "Undefined" "OverrideRootScale" null null)) ; プレイヤーアクターを生成する
  (`Controller.Possess` (`GameplayStatics.GetPlayerController` 0) _returnvalue) ; ポーンを所有する
  (`self.RespawnEvent`))

(fn `UserConstructionScript`)